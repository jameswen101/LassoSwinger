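; BP_Gate is a gate actor that raises and lowers when triggered through its BPIGate interface event.
; Each call flips an Open flag and plays or reverses the GateOpen timeline.
; The timeline lerps the actor between its stored starting position and a point Height units above it, calling a gate sound at its location on every update.
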(event EventBeginPlay
  (Variables|Default|SetStarting%20Position (Transformation|GetActorLocation)))

(event EventBPIGate
  (bind _starting_position (Variables|Default|GetStarting%20Position))
  ;[1 1 1] Keeps track of if the gate is open or closed
  (if (Variables|Default|GetOpen)
    (Variables|Default|SetOpen false)
    ;[1 1 1] Moves the gate between the start and end position
    (bind _alpha (Timeline|Gate%20Open Reverse)
      (:Update
        (Audio|PlaySoundatLocation "/Game/SFX/tanweraman-grave-yard-iron-gate-opening-392362.tanweraman-grave-yard-iron-gate-opening-392362" (Transformation|GetActorLocation) "0, 0, 0" 0.1 1.0 0.0 0 0 0 0)
        (Transformation|SetActorLocation (Math|Vector|Lerp(Vector) _starting_position (+ _starting_position (Math|Vector|MakeVector 0.0 0.0 (Variables|Default|GetHeight))) _alpha) false false)))
    (else
      (Variables|Default|SetOpen true)
      (Timeline|Gate%20Open Play))))

(fn ConstructionScript
  (Variables|Default|SetStarting%20Position (Transformation|GetActorLocation)))